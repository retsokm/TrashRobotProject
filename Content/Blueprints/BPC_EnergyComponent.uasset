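; Energy component for a BP_Robot, which drains energy while the robot moves and recharges it while it stands still.
; A looping timer started at BeginPlay applies the drain, and StartRegenEnergy starts a second timer that regenerates until full.
; Each energy change sends the normalized level to the robot through CallEnergyUpdated.
; Starting and stopping regeneration toggles the IsChargingEnergy key on the AI controller's blackboard.
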(event EventBeginPlay
  (bind _asbp_robot (Utilities|Casting|CastToBP_Robot (Components|GetOwner)))
  (bind _output_get (Variables|Default|SetBPRobotRef _asbp_robot))
  (bind _asaicontroller (Utilities|Casting|CastToAIController (Pawn|GetController _output_get)))
  (Variables|Default|SetAIControllerRef _asaicontroller)
  (Variables|Default|SetCurrentEnergy (Variables|Default|GetMaxEnergy))
  (bind _returnvalue (Utilities|Time|SetTimerbyFunctionName 0 "DrainEnergy" (Variables|Default|GetEnergyTickFrequency) true))
  (Variables|Default|SetEnergyDrainTimer _returnvalue))

(fn DrainEnergy
  (if (> (Math|Vector|VectorLength (Transformation|GetVelocity (Components|GetOwner))) 3.0)
    (bind _output_get (Variables|Default|SetCurrentEnergy (Math|Float|Clamp(Float) (- (Variables|Default|GetCurrentEnergy) (* (Variables|Default|GetEnergyCostPerSecond) (Variables|Default|GetEnergyTickFrequency))) 0.0 (Variables|Default|GetMaxEnergy))))
    (Default|CallEnergyUpdated (Variables|Default|GetBPRobotRef) (/ _output_get (Variables|Default|GetMaxEnergy)))))

(fn RegenEnergy
  (if (== (Math|Vector|VectorLength (Transformation|GetVelocity (Components|GetOwner))) 0.0)
    (bind _output_get (Variables|Default|SetCurrentEnergy (Math|Float|Clamp(Float) (+ (Variables|Default|GetCurrentEnergy) (* (Variables|Default|GetEnergyRegenPerSecond) (Variables|Default|GetEnergyTickFrequency))) 0.0 (Variables|Default|GetMaxEnergy))))
    (Default|CallEnergyUpdated (Variables|Default|GetBPRobotRef) (/ _output_get (Variables|Default|GetMaxEnergy)))
    (if (== (Variables|Default|GetCurrentEnergy) (Variables|Default|GetMaxEnergy))
      (CallFunction|StopRegenEnergy))))

(fn StartRegenEnergy
  (bind _returnvalue (Utilities|Time|SetTimerbyFunctionName 0 "RegenEnergy" (Variables|Default|GetEnergyTickFrequency) true))
  (Variables|Default|SetEnergyRegenTimer _returnvalue)
  (AI|Components|Blackboard|SetValueasBool (AI|GetBlackboard (Variables|Default|GetAIControllerRef)) (Utilities|Name|MakeLiteralName "IsChargingEnergy") true))

(fn StopRegenEnergy
  (Utilities|Time|ClearTimerbyFunctionName 0 "RegenEnergy")
  (AI|Components|Blackboard|SetValueasBool (AI|GetBlackboard (Variables|Default|GetAIControllerRef)) (Utilities|Name|MakeLiteralName "IsChargingEnergy") false))