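; Actor component that tracks how much trash a BP_Robot carries and handles gaining and releasing it.
; GainTrash adds a clamped amount per unit, and a looping timer drains it only while the owner stands still, stopping when empty.
; Changes are sent to the robot as a normalized fill ratio.
; Starting and stopping release sets the IsReleasingTrash blackboard key on the robot's AI controller.
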(event EventBeginPlay
  (bind _asbp_robot (Utilities|Casting|CastToBP_Robot (Components|GetOwner)))
  (bind _output_get (Variables|Default|SetBPRobotRef _asbp_robot))
  (bind _asaicontroller (Utilities|Casting|CastToAIController (Pawn|GetController _output_get)))
  (Variables|Default|SetAIControllerRef _asaicontroller))

(fn GainTrash
  (bind _output_get (Variables|Default|SetCurrentTrash (Math|Float|Clamp(Float) (+ (Variables|Default|GetCurrentTrash) (Variables|Default|GetTrashAmountPerUnit)) 0.0 (Variables|Default|GetMaxTrash))))
  (Default|CallTrashUpdated (Variables|Default|GetBPRobotRef) (/ _output_get (Variables|Default|GetMaxTrash))))

(fn ReleaseTrash
  (if (== (Math|Vector|VectorLength (Transformation|GetVelocity (Components|GetOwner))) 0.0)
    (bind _output_get (Variables|Default|SetCurrentTrash (Math|Float|Clamp(Float) (- (Variables|Default|GetCurrentTrash) (* (Variables|Default|GetTrashReleasePerSecond) (Variables|Default|GetTrashTickFrequency))) 0.0 (Variables|Default|GetMaxTrash))))
    (Default|CallTrashUpdated (Variables|Default|GetBPRobotRef) (/ _output_get (Variables|Default|GetMaxTrash)))
    (if (== (Variables|Default|GetCurrentTrash) 0.0)
      (CallFunction|StopReleaseTrash))))

(fn StartReleaseTrash
  (bind _returnvalue (Utilities|Time|SetTimerbyFunctionName 0 "ReleaseTrash" (Variables|Default|GetTrashTickFrequency) true))
  (Variables|Default|SetTrashReleaseTimer _returnvalue)
  (AI|Components|Blackboard|SetValueasBool (AI|GetBlackboard (Variables|Default|GetAIControllerRef)) (Utilities|Name|MakeLiteralName "IsReleasingTrash") true))

(fn StopReleaseTrash
  (Utilities|Time|ClearTimerbyFunctionName 0 "ReleaseTrash")
  (AI|Components|Blackboard|SetValueasBool (AI|GetBlackboard (Variables|Default|GetAIControllerRef)) (Utilities|Name|MakeLiteralName "IsReleasingTrash") false))