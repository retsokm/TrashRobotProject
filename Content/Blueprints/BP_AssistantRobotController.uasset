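; AI controller for the assistant robot that drives its behavior through a behavior tree.
; On BeginPlay it runs BT_AssistantRobot, then fills in the blackboard.
; It stores the controlled pawn's initial location and rotation as the robot's start transform keys, making them available to the tree.
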(event EventBeginPlay
  (AI|RunBehaviorTree "/Game/Blueprints/BT_AssistantRobot.BT_AssistantRobot")
  (CallFunction|SetupBlackboardValues))

(fn ConstructionScript)

(fn SetupBlackboardValues
  (AI|Components|Blackboard|SetValueasVector (AI|GetBlackboard 0) (Utilities|Name|MakeLiteralName "AssistantRobotStartLocation") (Transformation|GetActorLocation (Pawn|GetControlledPawn)))
  (Class|BlackboardComponent|SetValueasRotator (AI|GetBlackboard 0) (Utilities|Name|MakeLiteralName "AssistantRobotStartRotation") (Transformation|GetActorRotation (Pawn|GetControlledPawn))))