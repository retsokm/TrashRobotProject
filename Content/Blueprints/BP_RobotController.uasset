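; AI controller for a robot pawn that runs the BT_Robot behavior tree on BeginPlay.
; After starting the tree, it seeds the blackboard with the controlled pawn's starting location and rotation.
; It also stores the locations of the energy regen and trash release areas, each found with GetActorOfClass, so it uses a single actor of each type.
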(event EventBeginPlay
  (AI|RunBehaviorTree "/Game/Blueprints/BT_Robot.BT_Robot")
  (CallFunction|SetupBlackboardValues))

(fn ConstructionScript)

(fn SetupBlackboardValues
  (AI|Components|Blackboard|SetValueasVector (AI|GetBlackboard 0) (Utilities|Name|MakeLiteralName "RobotStartLocation") (Transformation|GetActorLocation (Pawn|GetControlledPawn)))
  (Class|BlackboardComponent|SetValueasRotator (AI|GetBlackboard 0) (Utilities|Name|MakeLiteralName "RobotStartRotation") (Transformation|GetActorRotation (Pawn|GetControlledPawn)))
  (bind _returnvalue (Actor|GetActorOfClass "/Game/Blueprints/BP_EnergyRegenArea.BP_EnergyRegenArea_C"))
  (AI|Components|Blackboard|SetValueasVector (AI|GetBlackboard 0) (Utilities|Name|MakeLiteralName "EnergyRegenAreaLocation") (Transformation|GetActorLocation _returnvalue))
  (bind _returnvalue_2 (Actor|GetActorOfClass "/Game/Blueprints/BP_TrashReleaseArea.BP_TrashReleaseArea_C"))
  (AI|Components|Blackboard|SetValueasVector (AI|GetBlackboard 0) (Utilities|Name|MakeLiteralName "TrashReleaseAreaLocation") (Transformation|GetActorLocation _returnvalue_2)))