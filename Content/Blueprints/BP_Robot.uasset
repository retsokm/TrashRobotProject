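; AI-controlled robot character that tracks energy and trash through components and exposes its settings to the player HUD.
; On BeginPlay it registers itself as owner of the HUD settings panel and its progress bar widget, fills the panel from component and movement values, and stores its start transform.
; Reset restores that transform, refills energy, empties trash, notifies of both changes, and clears the emergency and wander Blackboard flags, unchecking the wander checkbox.
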(event Custom|SetupPlayerUI
  (bind _asplayer_hud (Utilities|Casting|CastToPlayerHUD (HUD|GetHUD (Game|GetPlayerController 0))))
  (bind _output_get (Variables|Default|SetPlayerHUDRef _asplayer_hud))
  (Class|BPIUIOwner|SetUIOwner(Message) (Variables|/Game/HUD/PlayerHUD.PlayerHUD_C|GetRobotSettingsHUDRef _output_get) self)
  (CallFunction|SetupRobotSettingsValues))

(event Custom|SetupRoboterUI
  (Class|BPIUIOwner|SetUIOwner(Message) (UserInterface|GetUserWidgetObject (Variables|Default|GetProgressBarWidget)) self))

(event EventBeginPlay
  (CallFunction|SetupPlayerUI)
  (CallFunction|SetupRoboterUI)
  (Variables|Default|SetRobotStartTransform (Transformation|GetActorTransform)))

(event EventReset
  (bind _bpc_energycomponent (Variables|Default|GetBPC_EnergyComponent))
  (Transformation|SetActorTransform (Variables|Default|GetRobotStartTransform))
  (Variables|/Game/Blueprints/BPC_EnergyComponent.BPC_EnergyComponent_C|SetCurrentEnergy _bpc_energycomponent (Variables|/Game/Blueprints/BPC_EnergyComponent.BPC_EnergyComponent_C|GetMaxEnergy _bpc_energycomponent))
  (Default|CallEnergyUpdated 1.0)
  (Variables|/Game/Blueprints/BPC_TrashComponent.BPC_TrashComponent_C|SetCurrentTrash (Variables|Default|GetBPC_TrashComponent) 0.0)
  (Default|CallTrashUpdated 0.0)
  (bind _asaicontroller (Utilities|Casting|CastToAIController (Pawn|GetController)))
  (AI|Components|Blackboard|SetValueasBool (AI|GetBlackboard _asaicontroller) (Utilities|Name|MakeLiteralName "HasAnEmergency") false)
  (AI|Components|Blackboard|SetValueasBool (AI|GetBlackboard _asaicontroller) (Utilities|Name|MakeLiteralName "IsWanderActive") false)
  (Default|UpdateWCheckbox (Variables|/Game/HUD/PlayerHUD.PlayerHUD_C|GetRobotSettingsHUDRef (Variables|Default|GetPlayerHUDRef)) "Unchecked"))

(fn ConstructionScript)

(fn SetupRobotSettingsValues
  (Utilities|FlowControl|Sequence
    (:then_0
      (Default|UpdateLETText (Variables|/Game/HUD/PlayerHUD.PlayerHUD_C|GetRobotSettingsHUDRef (Variables|Default|GetPlayerHUDRef)) (Utilities|Text|ToText(Float) (Variables|/Game/Blueprints/BPC_EnergyComponent.BPC_EnergyComponent_C|GetLowEnergyTreshhold (Variables|Default|GetBPC_EnergyComponent)) "HalfToEven")))
    (:then_1
      (Default|UpdateECPSText (Variables|/Game/HUD/PlayerHUD.PlayerHUD_C|GetRobotSettingsHUDRef (Variables|Default|GetPlayerHUDRef)) (Utilities|Text|ToText(Float) (Variables|/Game/Blueprints/BPC_EnergyComponent.BPC_EnergyComponent_C|GetEnergyCostPerSecond (Variables|Default|GetBPC_EnergyComponent)) "HalfToEven")))
    (:then_2
      (Default|UpdateERPSText (Variables|/Game/HUD/PlayerHUD.PlayerHUD_C|GetRobotSettingsHUDRef (Variables|Default|GetPlayerHUDRef)) (Utilities|Text|ToText(Float) (Variables|/Game/Blueprints/BPC_EnergyComponent.BPC_EnergyComponent_C|GetEnergyRegenPerSecond (Variables|Default|GetBPC_EnergyComponent)) "HalfToEven")))
    (:then_3
      (Default|UpdateTRPSText (Variables|/Game/HUD/PlayerHUD.PlayerHUD_C|GetRobotSettingsHUDRef (Variables|Default|GetPlayerHUDRef)) (Utilities|Text|ToText(Float) (Variables|/Game/Blueprints/BPC_TrashComponent.BPC_TrashComponent_C|GetTrashReleasePerSecond (Variables|Default|GetBPC_TrashComponent)) "HalfToEven")))
    (:then_4
      (Default|UpdateTAPUText (Variables|/Game/HUD/PlayerHUD.PlayerHUD_C|GetRobotSettingsHUDRef (Variables|Default|GetPlayerHUDRef)) (Utilities|Text|ToText(Float) (Variables|/Game/Blueprints/BPC_TrashComponent.BPC_TrashComponent_C|GetTrashAmountPerUnit (Variables|Default|GetBPC_TrashComponent)) "HalfToEven")))
    (:then_5
      (Default|UpdateRSText (Variables|/Game/HUD/PlayerHUD.PlayerHUD_C|GetRobotSettingsHUDRef (Variables|Default|GetPlayerHUDRef)) (Utilities|Text|ToText(Float) (Variables|/Script/Engine.CharacterMovementComponent|GetMaxWalkSpeed (Variables|Character|GetCharacterMovement)) "HalfToEven")))
    (:then_6
      (Default|UpdateRSACheckbox (Variables|/Game/HUD/PlayerHUD.PlayerHUD_C|GetRobotSettingsHUDRef (Variables|Default|GetPlayerHUDRef)) (select (Variables|/Script/Engine.CharacterMovementComponent|GetbRequestedMoveUseAcceleration (Variables|Character|GetCharacterMovement)) "Checked" "Unchecked")))
    (:then_7
      (Default|UpdateELText (Variables|/Game/HUD/PlayerHUD.PlayerHUD_C|GetRobotSettingsHUDRef (Variables|Default|GetPlayerHUDRef)) (Utilities|Text|ToText(Float) (Variables|/Game/Blueprints/BPC_EnergyComponent.BPC_EnergyComponent_C|GetCurrentEnergy (Variables|Default|GetBPC_EnergyComponent)) "HalfToEven")))
    (:then_8
      (Default|UpdateTLText (Variables|/Game/HUD/PlayerHUD.PlayerHUD_C|GetRobotSettingsHUDRef (Variables|Default|GetPlayerHUDRef)) (Utilities|Text|ToText(Float) (Variables|/Game/Blueprints/BPC_TrashComponent.BPC_TrashComponent_C|GetCurrentTrash (Variables|Default|GetBPC_TrashComponent)) "HalfToEven")))))